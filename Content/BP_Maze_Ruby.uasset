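; BP_Maze_Ruby is a ruby pickup for the maze player.
; Its CollisionBox handles both overlap and hit events with identical logic, each reacting only when the other actor casts to BP_Maze_Player.
; On contact it prints a debug "Hello", calls CollectRubies on that player's PlayerController, then destroys itself.
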(event `self.CollisionBox.OnComponentBeginOverlap`
  (params (OverlappedComponent :type "PrimitiveComponent Object Reference") (OtherActor :type "Actor Object Reference") (OtherComp :type "PrimitiveComponent Object Reference") (OtherBodyIndex :type Integer) (bFromSweep :type Boolean) (SweepResult :type "HitResult Structure (by ref)"))
  (bind _asbp_maze_player (cast `/Game/BP_Maze_Player` OtherActor))
  (`KismetSystemLibrary.PrintString` "Hello")
  (`Maze_PlayerController.CollectRubies` (`Maze_Player.PlayerController` _asbp_maze_player))
  (`self.K2_DestroyActor`))

(event `self.CollisionBox.OnComponentHit`
  (params (HitComponent :type "PrimitiveComponent Object Reference") (OtherActor :type "Actor Object Reference") (OtherComp :type "PrimitiveComponent Object Reference") (NormalImpulse :type "Vector Structure") (Hit :type "HitResult Structure (by ref)"))
  (bind _asbp_maze_player (cast `/Game/BP_Maze_Player` OtherActor))
  (`KismetSystemLibrary.PrintString` "Hello")
  (`Maze_PlayerController.CollectRubies` (`Maze_Player.PlayerController` _asbp_maze_player))
  (`self.K2_DestroyActor`))

(fn `UserConstructionScript`)