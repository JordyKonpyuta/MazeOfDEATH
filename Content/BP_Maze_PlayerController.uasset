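; Player controller for a maze game that owns the main HUD widget and shows the ruby count.
; On BeginPlay it creates WBP_Main, gives it a reference to the controller, stores it and adds it to the viewport.
; The UpdateUI event pushes the controller's RubiesCount into the widget's text field, so the display refreshes only when that event is called.
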(event `self.ReceiveBeginPlay`
  (bind _returnvalue (`|CreateWidget` "/Game/WBP_Main.WBP_Main_C"))
  (set `/Game/WBP_Main.ControllerRef` self _returnvalue)
  (bind _output_get (set `self.UI_Ref` _returnvalue))
  (`UserWidget.AddToViewport` _output_get 0))

(event `self.UpdateUI`
  (`TextBlock.SetText` (`/Game/WBP_Main.Text_RubiesCount` (`self.UI_Ref`)) (`KismetTextLibrary.Conv_IntToText` (`self.RubiesCount`))))

(fn `UserConstructionScript`)