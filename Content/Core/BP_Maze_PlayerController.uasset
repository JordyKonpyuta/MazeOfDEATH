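; Player controller for a ruby-collecting maze game that manages its screens, HUD updates and end-of-game flow.
; It shows a loading screen on BeginPlay, opens the pause widget on P or Escape and refreshes the ruby count through UIRef.
; GameWon triggers the all-rubies UI and a looping one-second countdown that shows the victory screen when it runs out.
; GameOver pauses game and countdown, swaps music for a sound cue and shows the game-over screen.
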(event `self.ReceiveBeginPlay`
  ;[1 1 1] Begin play
  (bind _returnvalue (`|CreateWidget` "/Game/Core/Widgets/WBP_LoadingScreen.WBP_LoadingScreen_C"))
  (`UserWidget.AddToViewport` _returnvalue 0))

(event `self.UpdateUI`
  ;[1 1 1] Update UI
  (`TextBlock.SetText` (`/Game/Core/Widgets/WBP_Main.Text_RubiesCount` (`self.UI_Ref`)) (`KismetTextLibrary.Conv_IntToText` (`self.RubiesCount`))))

(event `Key|P`
  (params (Key :type "Key Structure"))
  ;[1 1 1] Pause Menu
  (:`Pressed`
    (bind _returnvalue (`|CreateWidget` "/Game/Core/Widgets/WBP_Pause.WBP_Pause_C" :!label _label))
    (`UserWidget.AddToViewport` _returnvalue 0)))

(event `Key|Escape`
  (params (Key :type "Key Structure"))
  ;[1 1 1] Pause Menu
  (:`Pressed`
    (goto _label)))

(event `self.GameWon`
  ;[1 1 1] Game Won
  (`/Game/Core/Widgets/WBP_Main.GotAllRubies_Start` (`self.UI_Ref`))
  (bind _returnvalue (`KismetSystemLibrary.K2_SetTimerDelegate` (delegate `SetTimer`) 1.0 true))
  (set `self.TimerRef` _returnvalue))

(event `SetTimer`
  ;[1 1 1] Game Won
  (if (> (`self.Timer`) 0.0)
    (`/Engine/EditorBlueprintResources/StandardMacros.DecrementFloat` (`self.Timer`)
      (:`  `
        (`TextBlock.SetText` (`/Game/Core/Widgets/WBP_Main.Text_Timer` (`self.UI_Ref`)) (`KismetTextLibrary.Conv_DoubleToText` (`self.Timer`) "HalfToEven"))))
    (else
      (`KismetSystemLibrary.K2_PauseTimerHandle` (`self.TimerRef`))
      (bind _returnvalue (`|CreateWidget` "/Game/Core/Widgets/WBP_VictoryScreen.WBP_VictoryScreen_C"))
      (`UserWidget.AddToViewport` _returnvalue 0))))

(event `self.GameOver`
  ;[1 1 1] Game Over
  (`GameplayStatics.SetGamePaused` true)
  (`KismetSystemLibrary.K2_PauseTimerHandle` (`self.TimerRef`))
  (`AudioComponent.Stop` (`/Game/Core/Widgets/WBP_Main.Music` (`self.UI_Ref`)))
  (`GameplayStatics.PlaySound2D` "/Game/Assets/Sounds/A_GameOver_Cue.A_GameOver_Cue" 1.0 1.0 0.0 null null)
  (bind _returnvalue (`|CreateWidget` "/Game/Core/Widgets/WBP_GameOver.WBP_GameOver_C"))
  (`UserWidget.AddToViewport` _returnvalue 0))

(fn `UserConstructionScript`)